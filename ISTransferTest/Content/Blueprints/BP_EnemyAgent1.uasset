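; Enemy agent Blueprint that chases the first player character and tracks whether it has reached them.
; BeginPlay starts an AI MoveTo on the player, repeating it after a short delay on each success; a failed move is not retried.
; Tick infers arrival from velocity alone: movement clears the reached and attacking flags, while any standstill sets reached.
; The attacking flag is never set true here.
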(event `self.ReceiveBeginPlay`
  (`|AIMoveTo` self (0.0 0.0 0.0) (`GameplayStatics.GetPlayerCharacter` 0) :!label _label
    (:`OnSuccess`
      (`KismetSystemLibrary.Delay` 0.2)
      (goto _label))))

(event `self.ReceiveTick`
  (params (DeltaSeconds :type "Float (single-precision)"))
  (if (> (`KismetMathLibrary.VSize` (`self.GetVelocity`)) 0.0)
    (set `self.m_playerReached` false)
    (set `self.m_isAttacking` false)
    (else
      (set `self.m_playerReached` true))))

(fn `UserConstructionScript`)